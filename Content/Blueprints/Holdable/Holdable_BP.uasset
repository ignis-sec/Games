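; Holdable physics object that the player's Ball_BP can attach to and release from, exchanging momentum with it.
; AttachPlayerToMe parents the ball's sphere to the Cylinder, applies incoming momentum as a force at the ball's center and removes linear damping.
; RemovePlayerFromMe samples the Cylinder's velocity at that point, detaches the sphere, restores damping and returns the velocity to the caller.
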(fn `AttachPlayerToMe`
  (params (Momentum :type "Vector Structure") (IsNegative :type Boolean))
  (bind _asball_bp (cast `/Game/Blueprints/Ball/Ball_BP` (`GameplayStatics.GetPlayerPawn` 0)))
  (bind _output_get (set `self.Sphere` (`/Game/Blueprints/Ball/Ball_BP.Sphere` _asball_bp)))
  (`SceneComponent.K2_AttachToComponent` _output_get (`self.Cylinder`) "None" "KeepWorld" "KeepWorld" "KeepWorld" true)
  (`PrimitiveComponent.AddForceAtLocation` (`self.Cylinder`) Momentum (`SceneComponent.K2_GetComponentLocation` (`/Game/Blueprints/Ball/Ball_BP.Ball_Center` _asball_bp)) "None")
  (`PrimitiveComponent.SetLinearDamping` (`self.Cylinder`) 0.0)
  (return))

(fn `RemovePlayerFromMe`
  (returns (Velocity :type "Vector Structure"))
  (bind _asball_bp (cast `/Game/Blueprints/Ball/Ball_BP` (`GameplayStatics.GetPlayerPawn` 0)))
  (bind _returnvalue (`PrimitiveComponent.GetPhysicsLinearVelocityAtPoint` (`self.Cylinder`) (`SceneComponent.K2_GetComponentLocation` (`/Game/Blueprints/Ball/Ball_BP.Ball_Center` _asball_bp)) "None"))
  (`SceneComponent.K2_DetachFromComponent` (`self.Sphere`) "KeepWorld" "KeepWorld" "KeepWorld" true)
  (`PrimitiveComponent.SetLinearDamping` (`self.Cylinder`) 1.0)
  (return _returnvalue))

(fn `UserConstructionScript`)