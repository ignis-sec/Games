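; Spawner actor that lays out an initial row of Holdable_BP actors at play start.
; A DoN loop with a delay spawns a fixed batch one at a time, stepping evenly along X at a fixed Y with random Z.
; Tick converts the player's ball X position into CurrentGrid, but no live logic here reads it.
; Seeded-random and position-based node checks are left disconnected.
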(event `self.ReceiveTick`
  (params (DeltaSeconds :type "Float (single-precision)"))
  (bind _returnvalue_x (`KismetMathLibrary.BreakVector` (`SceneComponent.K2_GetComponentLocation` (`/Game/Blueprints/Ball/Ball_BP.Ball_Center` (`self.Player`)))))
  (bind _output_get (set `self.CurrentGrid` (/ (`KismetMathLibrary.FFloor` _returnvalue_x) 150))))

(event `Initial Holdables`
  (bind _init_index (`self.Init_Index`))
  (`/Engine/EditorBlueprintResources/StandardMacros.Do N` 8 :!label _label
    (:`Exit`
      (`|SpawnActorFromClass` "/Game/Blueprints/Holdable/Holdable_BP.Holdable_BP_C" (`KismetMathLibrary.MakeTransform` (`KismetMathLibrary.MakeVector` (* _init_index 100.0) -40.0 (`KismetMathLibrary.Conv_IntToDouble` (`KismetMathLibrary.RandomIntegerInRange` -400 290)))) "AlwaysSpawn" "OverrideRootScale" null null)
      (`KismetSystemLibrary.PrintString` (`KismetStringLibrary.Concat_StrStr` "Spawned Actor " (`KismetStringLibrary.Conv_IntToString` _init_index)))
      (`/Engine/EditorBlueprintResources/StandardMacros.IncrementInt` (`self.Init_Index`)
        (:`  `
          (`KismetSystemLibrary.Delay` 1.0)
          (goto _label))))))

(event `self.ReceiveBeginPlay`
  (`self.Initial Holdables`))

(fn `UserConstructionScript`)