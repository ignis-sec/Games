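; Planet actor that randomizes its surface color and size, with all logic in the Construction Script and an inactive event graph.
; The script creates a dynamic instance of the planet material on the Body and sets a random RGB surface color.
; It then scales Body by a separate random value per axis, so shapes can be non-uniform and re-roll whenever construction reruns.
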(fn `UserConstructionScript`
  (bind _returnvalue (`KismetMathLibrary.RandomFloatInRange` 60.0 600.0))
  (if (!= (`self.Mat_Inst`) "/Game/Blueprints/Planets/Materials/MAT_Planet.MAT_Planet")
    (bind _returnvalue_2 (`KismetMaterialLibrary.CreateDynamicMaterialInstance` "/Game/Blueprints/Planets/Materials/MAT_Planet.MAT_Planet"))
    (bind _output_get (set `self.Mat_Inst` _returnvalue_2))
    (`PrimitiveComponent.SetMaterial` (`self.Body`) 0 _output_get))
  (`MaterialInstanceDynamic.SetVectorParameterValue` (`self.Mat_Inst`) "Surf_Color" (`KismetMathLibrary.MakeColor` (`KismetMathLibrary.RandomFloatInRange` 0.0 1.0) (`KismetMathLibrary.RandomFloatInRange` 0.0 1.0) (`KismetMathLibrary.RandomFloatInRange` 0.0 1.0) 1.0))
  (`SceneComponent.SetWorldScale3D` (`self.Body`) (`KismetMathLibrary.MakeVector` _returnvalue _returnvalue _returnvalue)))