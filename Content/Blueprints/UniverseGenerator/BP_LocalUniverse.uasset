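; Procedurally generates a local universe of stars with planets around the actor's position.
; On BeginPlay or CreateSelf, it seeds a random stream from the sum of its location coordinates, tying each layout to where it sits.
; CreateStar builds star data with randomized position, size, brightness and a list of randomized planets.
; Each entry becomes a BP_Stars child actor component, initialized by passing that data to its CreateSelf.
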(event `self.ReceiveBeginPlay`
  (bind (_returnvalue_x _returnvalue_y _returnvalue_z) (`KismetMathLibrary.BreakVector` (`self.K2_GetActorLocation`)))
  (`KismetMathLibrary.SetRandomStreamSeed` (`self.Seed`) (`KismetMathLibrary.FTrunc` (+ _returnvalue_x _returnvalue_y _returnvalue_z)) :!label _label)
  (for _ (range 1 (+ (`self.Number of Stars`) 1))
    (bind _star (`self.CreateStar`))
    (`KismetArrayLibrary.Array_Add` (`self.Stars`) _star))
  (for _array_element (`self.Stars`)
    (bind _returnvalue (`AddComponent|NODE_AddChildActorComponent-2`))
    (`ChildActorComponent.SetChildActorClass` _returnvalue "/Game/Blueprints/Stars/BP_Stars.BP_Stars_C")
    (bind _asbp_stars (cast `/Game/Blueprints/Stars/BP_Stars` (`ChildActorComponent.ChildActor` _returnvalue)))
    (`/Game/Blueprints/Stars/BP_Stars.CreateSelf` _asbp_stars _array_element)))

(event `Create Self`
  (goto _label))

(fn `CreateStar`
  (returns (Star :type "/Game/Data/ST_Star Structure"))
  (locals (Planets :type "Array of /Game/Data/ST_Planet Structure"))
  (bind (_distance _size _terrain_color _water_color _rotation) (`self.Create Planet`))
  (bind (_location _size_2 _brightness) (`self.Create Star`))
  (for _ (range (+ (`KismetMathLibrary.RandomIntegerInRangeFromStream` 0 (`self.MaxPlanetNumber`) (`self.Seed`)) 1))
    (`KismetArrayLibrary.Array_Add` (`local.Planets`) (make `/Game/Data/ST_Planet` _distance _size _rotation _terrain_color _water_color)))
  (return (make `/Game/Data/ST_Star` _location _size_2 (`local.Planets`) _brightness)))

(fn `UserConstructionScript`)