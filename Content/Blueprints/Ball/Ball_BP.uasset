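; Player ball for a side-scrolling rope-swing game, with an X-following camera, extending background and distance HUD.
; Left click attaches it to the Holdable nearest the cursor on screen, passing on its velocity; releasing restores velocity from that Holdable.
; While held, a per-tick line trace re-attaches the ball to any intervening Holdable, stacking previous ones in Tangled to fake rope wrapping.
; The rope is drawn with debug lines through those points.
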(event `Key|V`
  (params (Key :type "Key Structure"))
  (:`Pressed`
    (`GameplayStatics.OpenLevel` "Arcade")))

(event `self.ReceiveBeginPlay`
  (`self.Set Mouse Visiblity` true)
  (bind _returnvalue (`|CreateWidget` "/Game/HUD/Distance.Distance_C" (`GameplayStatics.GetPlayerController` 0)))
  (set `/Game/HUD/Distance.Player` self _returnvalue)
  (`UserWidget.AddToViewport` _returnvalue 0))

(event `Key|LeftMouseButton`
  (params (Key :type "Key Structure"))
  (bind _holded (`self.Holded`))
  ;[1 1 1] Clicking
  (:`Pressed`
    (bind _closest_holdable (`self.Get Closest Holdable`))
    (bind _output_get (set `self.Holded` _closest_holdable))
    (`self.HandlePhysicsTransfer` _output_get)
    (set `self.bIsHolding` true))
  (:`Released`
    (`PrimitiveComponent.SetMaterial` (`/Game/Blueprints/Holdable/Holdable_BP.Cylinder` _holded) 0 (`/Game/Blueprints/Holdable/Holdable_BP.Normal` _holded))
    (bind _velocity (`/Game/Blueprints/Holdable/Holdable_BP.RemovePlayerFromMe` _holded))
    (`PrimitiveComponent.SetPhysicsLinearVelocity` (`self.Sphere`) _velocity false "None")
    (set `self.bIsHolding` false)
    (`KismetArrayLibrary.Array_Clear` (`self.Tangled`))))

(event `self.ReceiveTick`
  (params (DeltaSeconds :type "Float (single-precision)"))
  (bind _holded (`self.Holded`))
  (bind _holded_2 (`self.Holded`))
  (`self.Set Camera Position`)
  (`self.Check and Extend BG`)
  (if (`self.bIsHolding`)
    (bind _outhit (`KismetSystemLibrary.LineTraceSingleForObjects` (`SceneComponent.K2_GetComponentLocation` (`self.Ball_Center`)) (`SceneComponent.K2_GetComponentLocation` (`/Game/Blueprints/Holdable/Holdable_BP.Cylinder` (`self.Holded`))) (`|MakeArray` "ObjectTypeQuery1" :!type "EObjectTypeQuery Enum")))
    (bind _asholdable_bp (cast `/Game/Blueprints/Holdable/Holdable_BP` (`.HitActor` (`GameplayStatics.BreakHitResult` _outhit))))
    (if (!= _asholdable_bp _holded_2)
      (bind _velocity (`/Game/Blueprints/Holdable/Holdable_BP.RemovePlayerFromMe` _holded_2))
      (`PrimitiveComponent.SetPhysicsLinearVelocity` (`self.Sphere`) _velocity false "None")
      (`PrimitiveComponent.SetMaterial` (`/Game/Blueprints/Holdable/Holdable_BP.Cylinder` _holded) 0 (`/Game/Blueprints/Holdable/Holdable_BP.Normal` _holded))
      (`KismetArrayLibrary.Array_Add` (`self.Tangled`) (`self.Holded`))
      (bind _output_get (set `self.Holded` _asholdable_bp))
      (`self.HandlePhysicsTransfer` _output_get)
      (`self.Manage Lines`)
      (else
        (`self.Manage Lines`)))))

(fn `Check and Extend BG`
  (if (`self.CheckBacgroundEndingDistance`)
    (`/Game/Blueprints/Background/BG_Actor.Extend Background` (`self.Background`))
    (return)))

(fn `Get Closest Holdable`
  (returns (`Closest Holdable` :type "/Game/Blueprints/Holdable/Holdable_BP Object Reference"))
  (set `self.Shortest Vector` 99999.0)
  (bind _returnvalue (`WidgetLayoutLibrary.GetMousePositionOnViewport`))
  (bind _outactors (`GameplayStatics.GetAllActorsOfClass` "/Game/Blueprints/Holdable/Holdable_BP.Holdable_BP_C"))
  (for (_array_element _array_index) _outactors
    (bind _returnvalue_2 (`KismetMathLibrary.VSize2D` (- (`GameplayStatics.ProjectWorldToScreen` (`GameplayStatics.GetPlayerController` 0) (`SceneComponent.K2_GetComponentLocation` (`/Game/Blueprints/Holdable/Holdable_BP.DefaultSceneRoot` _array_element)) true) _returnvalue)))
    (if (> (`self.Shortest Vector`) _returnvalue_2)
      (set `self.Shortest Vector` _returnvalue_2)
      (set `self.Shortest Index` _array_index)))
  (return (`|GetArrayItem` _outactors (`self.Shortest Index`))))

(fn `HandlePhysicsTransfer`
  (params (Holded :type "/Game/Blueprints/Holdable/Holdable_BP Object Reference"))
  (bind _returnvalue (`PrimitiveComponent.GetPhysicsLinearVelocity` (`self.Sphere`) "None"))
  (`PrimitiveComponent.SetMaterial` (`/Game/Blueprints/Holdable/Holdable_BP.Cylinder` Holded) 0 (`/Game/Blueprints/Holdable/Holdable_BP.Selected` Holded))
  (`/Game/Blueprints/Holdable/Holdable_BP.AttachPlayerToMe` Holded (* _returnvalue 100.0) false))

(fn `Manage Lines`
  (bind _tangled (`self.Tangled`))
  (bind _returnvalue (`KismetArrayLibrary.Array_Length` _tangled))
  (bind _returnvalue_2 (`KismetArrayLibrary.Array_Length` _tangled))
  ;[1 1 1] This Works Better
  (if (>= _returnvalue_2 2)
    (for _index (range (+ (- _returnvalue 2) 1))
      (`KismetSystemLibrary.DrawDebugLine` (`SceneComponent.K2_GetComponentLocation` (`/Game/Blueprints/Holdable/Holdable_BP.Cylinder` (`|GetArrayItem` _tangled _index))) (`SceneComponent.K2_GetComponentLocation` (`/Game/Blueprints/Holdable/Holdable_BP.Cylinder` (`|GetArrayItem` _tangled (+ _index 1)))) (struct :`R` 0.911458 :`B` 0.0068 :`A` 1.0) 0.0 5.0))
    (`KismetSystemLibrary.DrawDebugLine` (`SceneComponent.K2_GetComponentLocation` (`/Game/Blueprints/Holdable/Holdable_BP.Cylinder` (`|GetArrayItem` _tangled (- _returnvalue 1)))) (`SceneComponent.K2_GetComponentLocation` (`/Game/Blueprints/Holdable/Holdable_BP.Cylinder` (`self.Holded`))) (struct :`R` 0.911458 :`B` 0.0068 :`A` 1.0) 0.0 5.0 :!label _label)
    (elif (== _returnvalue_2 1)
      (goto _label)
      (else
        _)))
  (`KismetSystemLibrary.DrawDebugLine` (`SceneComponent.K2_GetComponentLocation` (`/Game/Blueprints/Holdable/Holdable_BP.Cylinder` (`self.Holded`))) (`SceneComponent.K2_GetComponentLocation` (`self.Ball_Center`)) (struct :`R` 0.911458 :`B` 0.0068 :`A` 1.0) 0.0 5.0))

(fn `Set Camera as Active`
  (`ActorComponent.SetActive` (`self.Camera1`) false false))

(fn `Set Camera Position`
  (bind _camera1 (`self.Camera1`))
  (bind _returnvalue_x (`KismetMathLibrary.BreakVector` (`SceneComponent.K2_GetComponentLocation` (`self.Sphere`))))
  (bind (_returnvalue_x_2 _returnvalue_y _returnvalue_z) (`KismetMathLibrary.BreakVector` (`SceneComponent.K2_GetComponentLocation` _camera1)))
  (`SceneComponent.K2_SetWorldLocation` _camera1 (`KismetMathLibrary.MakeVector` _returnvalue_x _returnvalue_y _returnvalue_z) false false)
  (return))

(fn `Set Mouse Visiblity`
  (params (Visiblity :type Boolean))
  (set `PlayerController.bShowMouseCursor` Visiblity (`GameplayStatics.GetPlayerController` 0))
  (return))

(fn `UserConstructionScript`)