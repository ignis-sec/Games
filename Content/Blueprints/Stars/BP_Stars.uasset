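; BP_Stars is a star actor that builds itself and its planets from an STStar struct.
; CreateSelf stores the struct, moves the actor, scales Body by Size and feeds Brightness into its Surf_Color material parameter as a grey value.
; CreatePlanets, a separate event, adds a BP_Planet child actor per planet entry, offset by Distance and rotated about Z.
; Each planet then initializes through its own CreateSelf with that entry.
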(event `CreateSelf`
  (params (ST_star :type "/Game/Data/ST_Star Structure"))
  (bind _output_get (set `self.ST_Star` ST_star))
  (`self.K2_SetActorLocation` (break `/Game/Data/ST_Star` _output_get))
  (`SceneComponent.SetWorldScale3D` (`self.Body`) (`KismetMathLibrary.MakeVector` (`.Size_5_4B1945D6400F8709DAAB0CB0F1391A68` (break `/Game/Data/ST_Star` _output_get)) (`.Size_5_4B1945D6400F8709DAAB0CB0F1391A68` (break `/Game/Data/ST_Star` _output_get)) (`.Size_5_4B1945D6400F8709DAAB0CB0F1391A68` (break `/Game/Data/ST_Star` _output_get))))
  (`MeshComponent.SetVectorParameterValueOnMaterials` (`self.Body`) "Surf_Color" (`KismetMathLibrary.MakeVector` (`.Brightness_11_EE2886CE44D3B0DFC29BAC8175CC271F` (break `/Game/Data/ST_Star` _output_get)) (`.Brightness_11_EE2886CE44D3B0DFC29BAC8175CC271F` (break `/Game/Data/ST_Star` _output_get)) (`.Brightness_11_EE2886CE44D3B0DFC29BAC8175CC271F` (break `/Game/Data/ST_Star` _output_get))))
  (`MeshComponent.SetVectorParameterValueOnMaterials` (`self.Body`) "Surf_Color" (`KismetMathLibrary.MakeVector` (`.Brightness_11_EE2886CE44D3B0DFC29BAC8175CC271F` (break `/Game/Data/ST_Star` _output_get)) (`.Brightness_11_EE2886CE44D3B0DFC29BAC8175CC271F` (break `/Game/Data/ST_Star` _output_get)) (`.Brightness_11_EE2886CE44D3B0DFC29BAC8175CC271F` (break `/Game/Data/ST_Star` _output_get)))))

(event `CreatePlanets`
  (bind (_st_star_location _st_star_size _st_star_planets) (break `/Game/Data/ST_Star` (`self.ST_Star`)))
  (for _array_element _st_star_planets
    (bind (_distance _size _rotation) (break `/Game/Data/ST_Planet` _array_element))
    (bind _returnvalue (`AddComponent|NODE_AddChildActorComponent-1` :`RelativeTransform` (`KismetMathLibrary.MakeTransform` (`KismetMathLibrary.RotateAngleAxis` (`KismetMathLibrary.MakeVector` _distance) _rotation (0.0 0.0 1.0)))))
    (bind _output_get (set `self.Child` _returnvalue))
    (`ChildActorComponent.SetChildActorClass` _output_get "/Game/Blueprints/Planets/BP_Planet.BP_Planet_C")
    (bind _asbp_planet (cast `/Game/Blueprints/Planets/BP_Planet` (`ChildActorComponent.ChildActor` _output_get)))
    (`/Game/Blueprints/Planets/BP_Planet.CreateSelf` _asbp_planet _array_element)))

(fn `UserConstructionScript`)