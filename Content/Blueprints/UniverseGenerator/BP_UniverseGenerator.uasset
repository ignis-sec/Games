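; BP_UniverseGenerator procedurally fills a universe with BP_Stars from a seeded random stream, attempting a set number on BeginPlay.
; CreateStar proceeds only when a random point lies within a threshold distance of the player, then draws a separate random location within the universe bounds.
; Each star becomes a child actor component, receiving an incrementing ID and generator reference before SpawnSet runs.
; A delayed clear-and-regenerate chain is disconnected.
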(event `self.ReceiveBeginPlay`
  (`KismetMathLibrary.SetRandomStreamSeed` (`self.Seed`) (`self.Seed For Universe`))
  (for _ (range 1 (+ (`self.Number of Stars`) 1))
    (`self.CreateStar` (`KismetMathLibrary.Conv_IntToDouble` (`self.Universe Radius`)))))

(fn `CreateStar`
  (params (`Universe Radius` :type "Float (double-precision)"))
  (bind _returnvalue (* `Universe Radius` -1.0))
  (bind _seed (`self.Seed`))
  (bind _returnvalue_2 (`KismetMathLibrary.MakeVector` (`KismetMathLibrary.RandomFloatInRangeFromStream` _returnvalue `Universe Radius` _seed) (`KismetMathLibrary.RandomFloatInRangeFromStream` _returnvalue `Universe Radius` _seed) (`KismetMathLibrary.RandomFloatInRangeFromStream` _returnvalue `Universe Radius` _seed)))
  (if (not (> (`KismetMathLibrary.VSize` (- (`self.K2_GetActorLocation` (`GameplayStatics.GetPlayerPawn` 0)) _returnvalue_2)) 10000.0))
    (bind _returnvalue_3 (`AddComponent|NODE_AddChildActorComponent-0` :`RelativeTransform` (`KismetMathLibrary.MakeTransform` _returnvalue_2)))
    (`ChildActorComponent.SetChildActorClass` _returnvalue_3 "/Game/Blueprints/Stars/BP_Stars.BP_Stars_C")
    (bind _asbp_stars (cast `/Game/Blueprints/Stars/BP_Stars` (`ChildActorComponent.ChildActor` _returnvalue_3)))
    (set `/Game/Blueprints/Stars/BP_Stars.StarID` (`self.CURID`) _asbp_stars)
    (set `self.CURID` (+ (`self.CURID`) 1))
    (set `/Game/Blueprints/Stars/BP_Stars.Universe` self _asbp_stars)
    (`/Game/Blueprints/Stars/BP_Stars.SpawnSet` _asbp_stars)))

(fn `UserConstructionScript`)