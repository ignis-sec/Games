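; BP_Universe streams BP_LocalUniverse chunks around the player in a 3D grid.
; Each tick it scans a block of cells offset from GetPlayerGrid, spawning child actors at unrecorded positions and calling CreateSelf.
; After each spawn, it culls chunks beyond three UniverseRadius from the player, using parallel location and component arrays.
; GetPlayerGrid's floored player-position calculations are unconnected in this graph.
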(event `self.ReceiveBeginPlay`)

(event `self.ReceiveTick`
  (params (DeltaSeconds :type "Float (single-precision)"))
  (bind _locals (`self.Locals`))
  (bind _childuniv (`self.ChildUniv`))
  (for _index (range -1 3)
    (for _index_2 (range -1 3)
      (for _index_3 (range -1 3)
        (bind _returnvalue (* (+ (+ (`self.GetPlayerGrid`) (2.0 2.0 2.0)) (`KismetMathLibrary.MakeVector` (`KismetMathLibrary.Conv_IntToDouble` _index) (`KismetMathLibrary.Conv_IntToDouble` _index_2) (`KismetMathLibrary.Conv_IntToDouble` _index_3))) 250000.0))
        (if (not (`KismetArrayLibrary.Array_Contains` _locals _returnvalue))
          (`KismetArrayLibrary.Array_Add` _locals _returnvalue)
          (bind _returnvalue_2 (`AddComponent|NODE_AddChildActorComponent-4` :`RelativeTransform` (`KismetMathLibrary.MakeTransform` _returnvalue)))
          (`KismetArrayLibrary.Array_Add` (`self.ChildUniv`) _returnvalue_2)
          (`ChildActorComponent.SetChildActorClass` _returnvalue_2 "/Game/Blueprints/UniverseGenerator/BP_LocalUniverse.BP_LocalUniverse_C")
          (bind _asbp_local_universe (cast `/Game/Blueprints/UniverseGenerator/BP_LocalUniverse` (`ChildActorComponent.ChildActor` _returnvalue_2)))
          (`/Game/Blueprints/UniverseGenerator/BP_LocalUniverse.Create Self` _asbp_local_universe)
          (for (_array_element _array_index) (`self.Locals`)
            (if (> (`KismetMathLibrary.VSize` (- (`self.K2_GetActorLocation` (`GameplayStatics.GetPlayerPawn` 0)) _array_element)) (* (`self.Universe Radius`) 3.0))
              (`KismetArrayLibrary.Array_RemoveItem` (`self.Locals`) _array_element)
              (bind _output (`|GetArrayItem` _childuniv _array_index))
              (`self.K2_DestroyActor` (`ChildActorComponent.ChildActor` _output))
              (`KismetArrayLibrary.Array_RemoveItem` _childuniv _output))))))))

(fn `UserConstructionScript`)