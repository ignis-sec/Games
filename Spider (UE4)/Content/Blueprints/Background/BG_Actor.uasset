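; BG_Actor is a Paper2D background actor that builds a horizontal strip of sprite tiles at runtime.
; On BeginPlay it calls ExtendBackground, which increments Iterator and adds Paper Sprite components for the indices from CurIterator up to it.
; Each scaled-up tile shows BG_Sprite and is offset along X by a fixed width times its index.
; CurIterator then stores the new end, so later calls continue the strip.
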(event `self.ReceiveBeginPlay`
  (`self.Extend Background`))

(fn `Extend Background`
  (bind _result (`/Engine/EditorBlueprintResources/StandardMacros.IncrementInt` (`self.Iterator`))
    (:`  `
      (for _index (range (`self.Cur_Iterator`) (+ _result 1))
        (bind _returnvalue (`AddComponent|NODE_AddPaperSpriteComponent-0` :`RelativeTransform` (`KismetMathLibrary.MakeTransform` (* (`KismetMathLibrary.MakeVector` 1280.0) _index) (struct) (2.0 2.0 2.0))))
        (`PaperSpriteComponent.SetSprite` _returnvalue "/Game/Blueprints/Background/BG_Sprite.BG_Sprite"))
      (set `self.Cur_Iterator` (`self.Iterator`))
      (return))))

(fn `UserConstructionScript`)